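; ChairProp_BP is a chair prop child Blueprint whose static mesh follows a type value.
; The construction script applies a fixed default entry from the ChairMesh map.
; SetNewType extends the parent's version, then looks up CurrentType in that map and swaps the mesh, or makes a TextRender visible when no entry exists.
; The event graph holds only disabled placeholder events.
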(fn `SetNewType`
  (params (NewType :type "/Game/SottoValentine/Blueprint/InteractabelObject/E_collectInteractable Enum" :default "NewEnumerator0"))
  (bind (_value _returnvalue) (`BlueprintMapLibrary.Map_Find` (`self.ChairMesh`) (`self.CurrentType`)))
  (`parent.SetNewType` NewType)
  (if _returnvalue
    (`StaticMeshComponent.SetStaticMesh` (`self.StaticMesh`) _value)
    (else
      (`SceneComponent.SetVisibility` (`self.TextRender`) true true))))

(fn `UserConstructionScript`
  (`parent.UserConstructionScript`)
  (`StaticMeshComponent.SetStaticMesh` (`self.StaticMesh`) (`BlueprintMapLibrary.Map_Find` (`self.ChairMesh`) "NewEnumerator6")))