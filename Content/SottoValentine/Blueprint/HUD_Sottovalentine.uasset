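; HUD actor for the SottoValentine game that creates the UI and hands off to the end game.
; On BeginPlay it shows the main character HUD and client selector widgets and binds to the game mode's 3D-game-ended event.
; That event opens the prop selector widget, whose confirmation calls PlayEndGame on the game mode.
; It then prints the selected chair, mirror and plant statuses for debugging.
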(event `self.ReceiveBeginPlay`
  (`|ExecutionSequence`
    (:`then_0`
      (bind _returnvalue (`|CreateWidget` "/Game/SottoValentine/Blueprint/UI/HUD_MainChar_BP.HUD_MainChar_BP_C" (`GameplayStatics.GetPlayerController` 0)))
      (`UserWidget.AddToViewport` _returnvalue 0)
      (bind _returnvalue_2 (`|CreateWidget` "/Game/SottoValentine/Blueprint/UI/UI_ClientSelector_BP.UI_ClientSelector_BP_C" (`GameplayStatics.GetPlayerController` 0)))
      (`UserWidget.AddToViewport` _returnvalue_2 0))
    (:`then_1`
      (bind _asbp_first_person_game_mode_sotto_valentine (cast `/Game/SottoValentine/Blueprint/BP_FirstPersonGameMode_SottoValentine` (`GameplayStatics.GetGameMode`)))
      (add `/Game/SottoValentine/Blueprint/BP_FirstPersonGameMode_SottoValentine.3DGameEnded` _asbp_first_person_game_mode_sotto_valentine (delegate `Start Prop Selection Menu`)))))

(event `Start Prop Selection Menu`
  (bind _returnvalue (`|CreateWidget` "/Game/SottoValentine/Blueprint/UI/UI_PropsSelector_BP.UI_PropsSelector_BP_C" (`GameplayStatics.GetPlayerController` 0)))
  (`UserWidget.AddToViewport` _returnvalue 0)
  (add `/Game/SottoValentine/Blueprint/UI/UI_PropsSelector_BP.SelectionConfirmed` _returnvalue (delegate `Play End Game`)))

(event `Play End Game`
  (`KismetSystemLibrary.PrintString` "PLAY END GAME")
  (bind _asbp_first_person_game_mode_sotto_valentine (cast `/Game/SottoValentine/Blueprint/BP_FirstPersonGameMode_SottoValentine` (`GameplayStatics.GetGameMode`)))
  (`/Game/SottoValentine/Blueprint/BP_FirstPersonGameMode_SottoValentine.PlayEndGame` _asbp_first_person_game_mode_sotto_valentine)
  (`KismetSystemLibrary.PrintString` (`|GetEnumeratorNameAsString` (`/Game/SottoValentine/Blueprint/BP_FirstPersonGameMode_SottoValentine.selectedChairStatus` _asbp_first_person_game_mode_sotto_valentine)))
  (`KismetSystemLibrary.PrintString` (`|GetEnumeratorNameAsString` (`/Game/SottoValentine/Blueprint/BP_FirstPersonGameMode_SottoValentine.selectedMirrorStatus` _asbp_first_person_game_mode_sotto_valentine)))
  (`KismetSystemLibrary.PrintString` (`|GetEnumeratorNameAsString` (`/Game/SottoValentine/Blueprint/BP_FirstPersonGameMode_SottoValentine.selectedPlantStatus` _asbp_first_person_game_mode_sotto_valentine))))

(fn `UserConstructionScript`)